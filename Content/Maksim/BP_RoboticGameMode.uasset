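; Game mode for a robotic arm fight that stages the intro between a player arm and an AI arm.
; BeginPlay finds both robots by tag and hides the enemy.
; StartGame blends the camera to the player, reveals and slides in the enemy, rotates the player's first part and shows both robots' widgets.
; After the slide and a short delay, StartFight activates the AI and possesses the player robot.
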(event Custom|Start%20Fight
  (Utilities|FlowControl|Delay 1.0)
  (Default|StartFight (Variables|Default|GetEnemy))
  (Pawn|Possess (Game|GetPlayerController 0) (Variables|Default|GetPlayerRobot)))

(event Custom|StartGame
  (Game|Player|SetViewTargetwithBlend (Game|GetPlayerController 0) (Variables|Default|GetPlayerRobot) 3.0 "VTBlend_Linear" 0.0 false)
  (Rendering|SetActorHiddenInGame (Variables|Default|GetEnemy) false)
  (Utilities|FlowControl|Sequence
    (:then_0
      (Components|MoveComponentTo (Variables|/Script/Engine.Actor|GetRootComponent (Variables|Default|GetEnemy)) "-180.000000,-830.000000,-220.000000" "0, 0, 0" true false 2.0 false)
      (CallFunction|StartFight))
    (:then_1
      (Components|MoveComponentTo (Variables|/Game/Maksim/BP_RoboticArm.BP_RoboticArm_C|Get1stPart (Variables|Default|GetPlayerRobot)) "0, 0, 0" "0,90.000000, 0" false false 2.0 true)
      (Development|SetHiddeninGame (Variables|/Game/Maksim/BP_RoboticArm.BP_RoboticArm_C|GetWidget (Variables|Default|GetEnemy)) false false))))

(event EventBeginPlay
  (Utilities|FlowControl|Sequence
    (:then_0
      (bind _outactors (Actor|GetAllActorswithTag "Enemy"))
      (bind _asbp_robotic_arm_ai (Utilities|Casting|CastToBP_RoboticArm_AI (Utilities|Array|Get(acopy) _outactors)))
      (bind _output_get (Variables|Default|SetEnemy _asbp_robotic_arm_ai))
      (Rendering|SetActorHiddenInGame _output_get true))
    (:then_1
      (bind _outactors_2 (Actor|GetAllActorswithTag "Player"))
      (bind _asbp_robotic_arm_player (Utilities|Casting|CastToBP_RoboticArm_Player (Utilities|Array|Get(acopy) _outactors_2)))
      (Variables|Default|SetPlayerRobot _asbp_robotic_arm_player))))

(fn ConstructionScript)