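; BP_PlayerController is the player controller that drives a possessed BP_RoboticArm from player input.
; On BeginPlay it casts the controlled pawn to BP_RoboticArm and caches the reference.
; Axis inputs yaw the arm's first segment in world space and rotate the wrist, both with fixed scaling.
; Attack and Block actions call the arm's start and stop functions on press and release.
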(event EventBeginPlay
  (bind _asbp_robotic_arm (Utilities|Casting|CastToBP_RoboticArm (Pawn|GetControlledPawn)))
  (Variables|Default|SetRobotic%20arm _asbp_robotic_arm))

(event Input|ActionEvents|InputActionAttack
  (params (Key :type Key%20Structure :default "None"))
  (bind _robotic_arm (Variables|Default|GetRobotic%20arm))
  (:Pressed
    (Default|AttackStart _robotic_arm))
  (:Released
    (Default|AttackStop _robotic_arm)))

(event Input|ActionEvents|InputActionBlock
  (params (Key :type Key%20Structure :default "None"))
  (bind _robotic_arm (Variables|Default|GetRobotic%20arm))
  (:Pressed
    (Default|StartBlocking _robotic_arm))
  (:Released
    (Default|StopBlocking _robotic_arm)))

(event Input|AxisEvents|InputAxisHorizontalRot
  (params (AxisValue :type Float%20%28single-precision%29))
  (Transformation|AddWorldRotation (Variables|/Game/Maksim/BP_RoboticArm.BP_RoboticArm_C|Get1stPart (Variables|Default|GetRobotic%20arm)) (Math|Rotator|MakeRotator 0.0 0.0 (* AxisValue 0.25)) false false))

(event Input|AxisEvents|InputAxisWristY
  (params (AxisValue :type Float%20%28single-precision%29))
  (Default|RotateWrist (Variables|Default|GetRobotic%20arm) (* AxisValue 6.0)))

(fn ConstructionScript)