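; Robotic arm Blueprint made of three jointed parts that plays a reversible attack motion.
; The construction script chains the parts from the base through sockets.
; AttackStart plays a timeline that pitches each joint, with the outer two sharing a derived angle, and AttackStop reverses it.
; HUD creation and blocking events are empty stubs.
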(event Custom|CreateHUD)

(event Custom|StartBlocking)

(event Custom|StopBlocking)

(event Custom|AttackStart
  (Utilities|FlowControl|Sequence
    (:then_0
      (bind _rot (Timeline|AttackTimeline Stop)
        (:Update
          (CallFunction|SetRelativeRotY (Variables|Default|Get1stPart) (* _rot -1.0))
          (CallFunction|SetRelativeRotY (Variables|Default|Get2ndPart) (/ (- 9e+01 _rot) -2.0))
          (CallFunction|SetRelativeRotY (Variables|Default|Get3rdPart) (/ (- 9e+01 _rot) -2.0)))))
    (:then_1
      (Timeline|AttackTimeline Play))))

(event Custom|AttackStop
  (Utilities|FlowControl|Sequence
    (:then_0
      (bind _rot (Timeline|AttackTimeline Stop)
        (:Update
          (CallFunction|SetRelativeRotY (Variables|Default|Get1stPart) (* _rot -1.0))
          (CallFunction|SetRelativeRotY (Variables|Default|Get2ndPart) (/ (- 9e+01 _rot) -2.0))
          (CallFunction|SetRelativeRotY (Variables|Default|Get3rdPart) (/ (- 9e+01 _rot) -2.0)))))
    (:then_1
      (Timeline|AttackTimeline Reverse))))

(event EventBeginPlay)

(event Collision|EventActorBeginOverlap
  (params (OtherActor :type Actor%20Object%20Reference)))

(event EventTick
  (params (DeltaSeconds :type Float%20%28single-precision%29)))

(fn ConstructionScript
  (Transformation|AttachComponentToComponent (Variables|Default|Get1stPart) (Variables|Default|GetBase) "AttachmentPoint" "KeepWorld" "KeepWorld" "KeepWorld" true)
  (Transformation|AttachComponentToComponent (Variables|Default|Get2ndPart) (Variables|Default|Get1stPart) "End" "KeepWorld" "KeepRelative" "KeepWorld" true)
  (Transformation|AttachComponentToComponent (Variables|Default|Get3rdPart) (Variables|Default|Get2ndPart) "End" "KeepWorld" "KeepRelative" "KeepWorld" true))

(fn SetRelativeRotY
  (params (Target :type Static%20Mesh%20Component%20Object%20Reference) (Pitch :type Float%20%28single-precision%29))
  (bind _relativerotation (Variables|/Script/Engine.SceneComponent|GetRelativeRotation Target))
  (Transformation|SetRelativeRotation Target (Math|Rotator|MakeRotator (.roll _relativerotation) Pitch (.yaw _relativerotation)) false false))