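; AI-driven robotic arm that fights other BP_RoboticArm actors, looping random attacks once StartFight fires.
; After a delay, NewAttack picks a vertical wrist swing or horizontal base sweep, each a timeline rotating components.
; Timeline event tracks toggle attacking, plus blocking during sweeps.
; Weapon overlap with another arm's weapon stops and reverses the current swing; hitting other parts of that arm applies damage.
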(event OnComponentBeginOverlap(Weapon)
  (params (OverlappedComponent :type Primitive%20Component%20Object%20Reference) (OtherActor :type Actor%20Object%20Reference) (OtherComp :type Primitive%20Component%20Object%20Reference) (OtherBodyIndex :type Integer) (bFromSweep :type Boolean) (SweepResult :type Hit%20Result%20Structure%20%28by%20ref%29))
  (bind _asbp_robotic_arm (Utilities|Casting|CastToBP_RoboticArm OtherActor))
  (if (== (Variables|/Game/Maksim/BP_RoboticArm.BP_RoboticArm_C|GetWeapon _asbp_robotic_arm) OtherComp)
    (CallFunction|StopDoingWhatYouDo)
    (else
      (Game|Damage|ApplyDamage OtherActor (Variables|Default|GetDamage) (Pawn|GetController) self "/Script/Engine.DamageType"))))

(event Custom|StartFight
  (CallFunction|NewAttack))

(event Custom|HorizontalAttack
  (bind _basez (Timeline|HorizontalAttackTimeline PlayFromStart)
    (:Update
      (Transformation|SetRelativeRotation (Variables|Default|Get1stPart) (Math|Rotator|CombineRotators (Variables|Default|GetBaseRelRotInit) (Math|Rotator|MakeRotator 0.0 0.0 (- _basez 9e+01))) false false))
    (:Finished
      (CallFunction|NewAttack))
    (:AttackTrack
      (CallFunction|AttackStart))
    (:StopAttackTrack
      (CallFunction|AttackStop))
    (:StopBlockTrack
      (CallFunction|StopBlocking))
    (:BlockTrack
      (CallFunction|StartBlocking))))

(event Custom|VerticalAttack
  (bind _wristy (Timeline|VerticalAttackTimeline PlayFromStart)
    (:Update
      (Transformation|SetRelativeRotation (Variables|Default|GetWrist) (Math|Rotator|CombineRotators (Variables|Default|GetWristRelRotInit) (Math|Rotator|MakeRotator 0.0 _wristy 0.0)) false false))
    (:Finished
      (CallFunction|NewAttack))
    (:AttackTrack
      (CallFunction|AttackStart))
    (:StopAttack
      (CallFunction|AttackStop))))

(event Custom|NewAttack
  (Utilities|FlowControl|Delay 2.0)
  (bind _output_get (Variables|Default|SetbPerformingVertAttack (Math|Random|RandomBool)))
  (if _output_get
    (CallFunction|VerticalAttack)
    (else
      (CallFunction|HorizontalAttack))))

(event Custom|StopDoingWhatYouDo
  (if (Variables|Default|GetbPerformingVertAttack)
    (Utilities|FlowControl|Sequence
      (:then_0
        (bind _wristy (Timeline|VerticalAttackTimeline Stop)
          (:Update
            (Transformation|SetRelativeRotation (Variables|Default|GetWrist) (Math|Rotator|CombineRotators (Variables|Default|GetWristRelRotInit) (Math|Rotator|MakeRotator 0.0 _wristy 0.0)) false false))
          (:Finished
            (CallFunction|NewAttack))
          (:AttackTrack
            (CallFunction|AttackStart))
          (:StopAttack
            (CallFunction|AttackStop))))
      (:then_1
        (Timeline|VerticalAttackTimeline Reverse))
      (:then_2
        (CallFunction|NewAttack)))
    (else
      (Utilities|FlowControl|Sequence
        (:then_0
          (bind _basez (Timeline|HorizontalAttackTimeline Stop)
            (:Update
              (Transformation|SetRelativeRotation (Variables|Default|Get1stPart) (Math|Rotator|CombineRotators (Variables|Default|GetBaseRelRotInit) (Math|Rotator|MakeRotator 0.0 0.0 (- _basez 9e+01))) false false))
            (:Finished
              (CallFunction|NewAttack))
            (:AttackTrack
              (CallFunction|AttackStart))
            (:StopAttackTrack
              (CallFunction|AttackStop))
            (:StopBlockTrack
              (CallFunction|StopBlocking))
            (:BlockTrack
              (CallFunction|StartBlocking))))
        (:then_1
          (Timeline|HorizontalAttackTimeline Reverse))))))

(event EventBeginPlay
  (|CallParentFunction))

(event EventDeath
  (Actor|DestroyActor))

(fn ConstructionScript
  (|CallParentFunction))