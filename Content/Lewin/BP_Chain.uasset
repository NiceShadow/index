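; Chain actor whose links, built as hierarchical instanced static meshes, move continuously along a spline.
; The construction script adds evenly spaced instances along the spline, all initially using the rotation at its start.
; A timeline restarted on finish drives Alpha, and each update offsets every link's distance by that fraction of the spline length.
; Links passing the end wrap to the start, taking location and rotation from the spline.
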(event EventBeginPlay
  (bind _newtrack_0 (Timeline|Timeline_0 PlayFromStart)
    (:Update
      (Variables|Default|SetAlpha _newtrack_0)
      (for _index (range 0 (- (Variables|Default|GetChainElementsAmount) 1))
        (CallFunction|TransformAChainElment _index)))
    (:Finished
      (Timeline|Timeline_0 PlayFromStart))))

(fn ConstructionScript
  (bind _spline (Variables|Default|GetSpline))
  (for _index (range 0 (- (Variables|Default|GetChainElementsAmount) 1))
    (Components|InstancedStaticMesh|AddInstance (Variables|Default|GetHierarchicalInstancedStaticMesh) (Math|Transform|MakeTransform (Spline|GetLocationatDistanceAlongSpline _spline (* _index (Variables|Default|GetDistanceBetweenElements)) "Local") (Spline|GetRotationatDistanceAlongSpline _spline 0.0 "Local") (Math|Conversions|ToVector(Float) (Variables|Default|GetMeshSize))))))

(fn TransformAChainElment
  (params (InstanceIndex :type Integer))
  (bind _spline (Variables|Default|GetSpline))
  (bind _spline_2 (Variables|Default|GetSpline))
  (bind _returnvalue (Spline|GetNumberOfSplinePoints _spline_2))
  (bind _returnvalue_2 (Spline|GetDistanceAlongSplineatSplinePoint _spline_2 _returnvalue))
  (LocalVariables|SetIndex InstanceIndex)
  (Components|InstancedStaticMesh|UpdateInstanceTransform (Variables|Default|GetHierarchicalInstancedStaticMesh) (LocalVariables|GetIndex) (Math|Transform|MakeTransform (Spline|GetLocationatDistanceAlongSpline _spline (Math|Float|SelectFloat (- (+ (Math|Float|Lerp 0.0 _returnvalue_2 (Variables|Default|GetAlpha)) (* (LocalVariables|GetIndex) (Variables|Default|GetDistanceBetweenElements))) _returnvalue_2) (+ (Math|Float|Lerp 0.0 _returnvalue_2 (Variables|Default|GetAlpha)) (* (LocalVariables|GetIndex) (Variables|Default|GetDistanceBetweenElements))) (> (+ (Math|Float|Lerp 0.0 _returnvalue_2 (Variables|Default|GetAlpha)) (* (LocalVariables|GetIndex) (Variables|Default|GetDistanceBetweenElements))) _returnvalue_2)) "Local") (Spline|GetRotationatDistanceAlongSpline _spline (Math|Float|SelectFloat (- (+ (Math|Float|Lerp 0.0 _returnvalue_2 (Variables|Default|GetAlpha)) (* (LocalVariables|GetIndex) (Variables|Default|GetDistanceBetweenElements))) _returnvalue_2) (+ (Math|Float|Lerp 0.0 _returnvalue_2 (Variables|Default|GetAlpha)) (* (LocalVariables|GetIndex) (Variables|Default|GetDistanceBetweenElements))) (> (+ (Math|Float|Lerp 0.0 _returnvalue_2 (Variables|Default|GetAlpha)) (* (LocalVariables|GetIndex) (Variables|Default|GetDistanceBetweenElements))) _returnvalue_2)) "Local") (Math|Conversions|ToVector(Float) (Variables|Default|GetMeshSize))) false false false))